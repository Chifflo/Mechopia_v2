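; Mr_Mushy is an enemy that chases the player and deals contact damage.
; Every tick it issues a simple move-to toward player 0 through its instigator controller, as long as that character is valid.
; When an overlap begins and the player is overlapping it, it calls TakingDamage on the MechopiaCharacter with its Damage value and prints the returned number.
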(event Collision|EventActorBeginOverlap
  (params (OtherActor :type Actor%20Object%20Reference))
  (bind _returnvalue (Game|GetPlayerCharacter 0))
  (if (Collision|IsOverlappingActor _returnvalue :!class /Script/Engine.Actor)
    (if true
      (bind _asmechopia_character (Utilities|Casting|CastToMechopiaCharacter _returnvalue))
      (Development|PrintText (Utilities|Text|ToText(Integer) (Class|MechopiaCharacter|TakingDamage _asmechopia_character (Variables|Default|GetDamage)))))))

(event EventTick
  (params (DeltaSeconds :type Float%20%28single-precision%29))
  (bind _returnvalue (Game|GetPlayerCharacter 0))
  (Utilities|IsValid _returnvalue
    (:Is%20Valid
      (AI|Navigation|SimpleMovetoActor (Game|GetInstigatorController) _returnvalue))))

(fn ConstructionScript)